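; Interactable door actor that swings open and closed each time its ActorDoes event fires.
; A DoorOpen flag picks between playing and reversing a timeline, whose track scales a fixed angle into the Door component's relative yaw.
; It also reports a NeedGift count as the gifts needed to interact and always returns true from ShouldTrack.
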(event EventBeginPlay)

(event Collision|EventActorBeginOverlap
  (params (OtherActor :type Actor%20Object%20Reference)))

(event EventTick
  (params (DeltaSeconds :type Float%20%28single-precision%29)))

(event EventActorDoes
  (params (Character :type BP%20Third%20Person%20Character%20Object%20Reference))
  (if (Variables|Default|GetDoorOpen)
    (Variables|Default|SetAngle 1.2e+02)
    (Variables|Default|SetDoorOpen false)
    (bind _newtrack_0 (Timeline|Timeline Reverse)
      (:Update
        (Transformation|SetRelativeRotation (Variables|Default|GetDoor) (Math|Rotator|MakeRotator 0.0 0.0 (* _newtrack_0 (Variables|Default|GetAngle))) false false)))
    (else
      (Variables|Default|SetAngle 1.2e+02)
      (Variables|Default|SetDoorOpen true)
      (Timeline|Timeline Play))))

(fn ConstructionScript)

(fn HowManyGiftNeededtoInteract
  (return (Variables|Default|GetNeedGift)))

(fn ShouldTrack
  (return true))