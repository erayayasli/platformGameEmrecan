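; BP_Gift is a collectible gift pickup that awards the player a point on contact.
; On BeginPlay it caches the player's BP_HUD.
; When a BP_ThirdPersonCharacter overlaps its Box, it increments that character's Point and pushes the new total to the HUD's WBPPoint widget.
; It then plays a 2D sound cue and destroys itself.
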(event OnComponentBeginOverlap(Box)
  (params (OverlappedComponent :type Primitive%20Component%20Object%20Reference) (OtherActor :type Actor%20Object%20Reference) (OtherComp :type Primitive%20Component%20Object%20Reference) (OtherBodyIndex :type Integer) (bFromSweep :type Boolean) (SweepResult :type Hit%20Result%20Structure%20%28by%20ref%29))
  (bind _asbp_third_person_character (Utilities|Casting|CastToBP_ThirdPersonCharacter OtherActor))
  (bind _output_get (Variables|/Game/_Game/Character/BP_ThirdPersonCharacter.BP_ThirdPersonCharacter_C|SetPoint _asbp_third_person_character (+ (Variables|/Game/_Game/Character/BP_ThirdPersonCharacter.BP_ThirdPersonCharacter_C|GetPoint _asbp_third_person_character) 1)))
  (Default|UpdatePoint (Variables|/Game/_Game/BP_HUD.BP_HUD_C|GetWBP_Point (Variables|Default|GetOurHUD)) _output_get)
  (Audio|PlaySound2D "/Game/KennyAssets/Audio/GiftCue.GiftCue" 1.0 1.0 0.0 0 0)
  (Actor|DestroyActor))

(event EventBeginPlay
  (bind _asbp_hud (Utilities|Casting|CastToBP_HUD (HUD|GetHUD (Game|GetPlayerController 0))))
  (Variables|Default|SetOurHUD _asbp_hud))

(fn ConstructionScript)