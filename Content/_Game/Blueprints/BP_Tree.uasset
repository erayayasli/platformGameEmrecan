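; BP_Tree is an interactable tree actor that holds a supply of apples as child components of its mesh.
; Each ActorDoes call, while apples remain, destroys the first child component and clears IsThereApple once none are left.
; HowManyGiftNeededToInteract returns the NeedGift requirement, and ShouldTrack reports whether apples remain.
; BeginPlay caches the player's BP_HUD, though this graph does not use it further.
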(event EventBeginPlay
  (bind _asbp_hud (Utilities|Casting|CastToBP_HUD (HUD|GetHUD (Game|GetPlayerController 0))))
  (Variables|Default|SetBP_HUD _asbp_hud))

(event EventActorDoes
  (params (Character :type BP%20Third%20Person%20Character%20Object%20Reference))
  (if (Variables|Default|GetIsThereApple)
    (Components|DestroyComponent (Components|GetChildComponent (Variables|Default|GetTreeMesh) 0))
    (if (== (Class|SceneComponent|GetNumChildrenComponents (Variables|Default|GetTreeMesh)) 0)
      (Variables|Default|SetIsThereApple false))))

(fn ConstructionScript)

(fn HowManyGiftNeededtoInteract
  (return (Variables|Default|GetNeedGift)))

(fn ShouldTrack
  (return (Variables|Default|GetIsThereApple)))